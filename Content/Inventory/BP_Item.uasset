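; BP_Item is an inventory item actor whose mesh, name and quest flag are driven by an item ID.
; The construction script linearly scans the ItemData table for a row with a matching ItemID, then copies its values onto the actor.
; Dropped assigns a new ID, calls CreateItem (body not shown), then MakeMeshCorrect, which applies ThisMesh to the static mesh component.
; The event graph holds only disabled placeholder events.
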(event EventBeginPlay)

(event Collision|EventActorBeginOverlap
  (params (OtherActor :type Actor%20Object%20Reference)))

(event EventTick
  (params (DeltaSeconds :type Float%20%28single-precision%29)))

(fn ConstructionScript
  (bind _outrownames (DataTable|GetDataTableRowNames "/Game/Inventory/ItemData.ItemData"))
  (for _array_element _outrownames
    (bind _returnvalue (Utilities|GetDataTableRow "/Game/Inventory/ItemData.ItemData" _array_element)
      (:then
        (if (== (.ItemID (Utilities|Struct|BreakItemData _returnvalue)) (Variables|Default|GetItemID))
          (Components|StaticMesh|SetStaticMesh (Variables|Default|GetStaticMeshComponent) (.Mesh (Utilities|Struct|BreakItemData _returnvalue)))
          (Variables|Default|SetITemName (.ItemName (Utilities|Struct|BreakItemData _returnvalue)))
          (Variables|Default|SetQuestItem (.IsQuestItem (Utilities|Struct|BreakItemData _returnvalue))))))))

(fn MakeMeshCorrect
  (Components|StaticMesh|SetStaticMesh (Variables|Default|GetStaticMeshComponent) (Variables|Default|GetThisMesh)))

(fn Dropped
  (params (ItemID :type Integer))
  (Variables|Default|SetItemID ItemID)
  (Class|Item|CreateItem)
  (CallFunction|MakeMeshCorrect))