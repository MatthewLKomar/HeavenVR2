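; Simplified VR character that poses its hands and pulls inventory items into the right hand.
; SetPointState and SetGripState turn trigger and grip input into hand animation poses, showing the widget interaction debug pointer only while gripping without trigger.
; ItemID spawns a weapon for certain IDs or a generic item otherwise, decrements inventory stock except for quest items, then attaches and grips it.
; The event graph contains no active logic.
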(event EventBeginPlay)

(event Collision|EventActorBeginOverlap
  (params (OtherActor :type Actor%20Object%20Reference)))

(event EventTick
  (params (DeltaSeconds :type Float%20%28single-precision%29)))

(fn ConstructionScript)

(fn SetPointState
  (params (Hand :type Skeletal%20Mesh%20Component%20Object%20Reference) (TriggerPressed :type Boolean) (GripPressed :type Boolean) (WidgetInteractor :type Widget%20Interaction%20Component%20Object%20Reference))
  (bind _asbp_hand_anim (Utilities|Casting|CastToBP_Hand_Anim (Components|SkeletalMesh|GetAnimInstance Hand)))
  (LocalVariables|SetHandAnim _asbp_hand_anim)
  (if TriggerPressed
    ;[1 1 1] What to do if we're pointing and are we gripping?
    (if GripPressed
      (Variables|/Game/Geometry/CustomHand/Anim/BP_Hand_Anim.BP_Hand_Anim_C|SetOpen (LocalVariables|GetHandAnim) 3.0)
      (else
        (Variables|/Game/Geometry/CustomHand/Anim/BP_Hand_Anim.BP_Hand_Anim_C|SetOpen (LocalVariables|GetHandAnim) 1.0)))
    (Utilities|IsValid WidgetInteractor
      (:Is%20Valid
        (Variables|/Script/UMG.WidgetInteractionComponent|SetbShowDebug WidgetInteractor false)))
    (elif GripPressed
      (Variables|/Game/Geometry/CustomHand/Anim/BP_Hand_Anim.BP_Hand_Anim_C|SetOpen (LocalVariables|GetHandAnim) 2.0)
      (Utilities|IsValid WidgetInteractor
        (:Is%20Valid
          (Variables|/Script/UMG.WidgetInteractionComponent|SetbShowDebug WidgetInteractor true)))
      (else
        (Variables|/Game/Geometry/CustomHand/Anim/BP_Hand_Anim.BP_Hand_Anim_C|SetOpen (LocalVariables|GetHandAnim) 0.0)
        (Utilities|IsValid WidgetInteractor
          (:Is%20Valid
            (Variables|/Script/UMG.WidgetInteractionComponent|SetbShowDebug WidgetInteractor false)))))))

(fn SetGripState
  (params (GripPressed :type Boolean) (TriggerPressed :type Boolean) (Hand :type Skeletal%20Mesh%20Component%20Object%20Reference) (WidgetInteraction :type Widget%20Interaction%20Component%20Object%20Reference))
  (bind _asbp_hand_anim (Utilities|Casting|CastToBP_Hand_Anim (Components|SkeletalMesh|GetAnimInstance Hand)))
  (LocalVariables|SetHandAnim _asbp_hand_anim)
  (if GripPressed
    (if TriggerPressed
      (Variables|/Game/Geometry/CustomHand/Anim/BP_Hand_Anim.BP_Hand_Anim_C|SetOpen (LocalVariables|GetHandAnim) 3.0)
      (Utilities|IsValid WidgetInteraction
        (:Is%20Valid
          (Variables|/Script/UMG.WidgetInteractionComponent|SetbShowDebug WidgetInteraction false :!label _label))
        (:Is%20Not%20Valid
          _))
      (else
        (Variables|/Game/Geometry/CustomHand/Anim/BP_Hand_Anim.BP_Hand_Anim_C|SetOpen (LocalVariables|GetHandAnim) 2.0)
        (Utilities|IsValid WidgetInteraction
          (:Is%20Valid
            (Variables|/Script/UMG.WidgetInteractionComponent|SetbShowDebug WidgetInteraction true))
          (:Is%20Not%20Valid
            _))))
    (elif TriggerPressed
      (Variables|/Game/Geometry/CustomHand/Anim/BP_Hand_Anim.BP_Hand_Anim_C|SetOpen (LocalVariables|GetHandAnim) 1.0)
      (Utilities|IsValid WidgetInteraction
        (:Is%20Valid
          (goto _label))
        (:Is%20Not%20Valid
          _))
      (else
        (Variables|/Game/Geometry/CustomHand/Anim/BP_Hand_Anim.BP_Hand_Anim_C|SetOpen (LocalVariables|GetHandAnim) 0.0)
        (Utilities|IsValid WidgetInteraction
          (:Is%20Valid
            (goto _label))
          (:Is%20Not%20Valid
            _)))))
  (return GripPressed))

(fn ItemID
  (params (ItemID :type Integer))
  (bind _inventory (Variables|Default|GetInventory))
  (bind _righthand (Variables|Default|GetRightHand))
  (bind _socketname (Variables|Default|GetSocketName))
  (bind _inventory_2 (Variables|Default|GetInventory))
  (bind _returnvalue (Transformation|GetSocketLocation _righthand _socketname))
  (bind _inventorystock (Variables|/Script/HeavenVR2.Inventory|GetInventoryStock _inventory))
  (bind _inventorystock_2 (Variables|/Script/HeavenVR2.Inventory|GetInventoryStock _inventory_2))
  (bind _returnvalue_2 (Math|Transform|MakeTransform _returnvalue))
  (switch int ItemID
    (:Default
      (bind _returnvalue_3 (Game|SpawnActorfromClass "/Game/Inventory/BP_Item.BP_Item_C" _returnvalue_2 "AlwaysSpawn" 0 0))
      (bind _output_get (LocalVariables|SetDroppedItem _returnvalue_3))
      (Default|Dropped _output_get ItemID)
      (for (_array_element _array_index) (Variables|/Script/HeavenVR2.Inventory|GetInventoryStock (Variables|Default|GetInventory))
        (if (== (.ID (Utilities|Struct|BreakItemSetting _array_element)) ItemID)
          ;[1 1 1] Remove Clues
          (if (not (Variables|/Script/HeavenVR2.Item|GetIsQuestItem (LocalVariables|GetDroppedItem)))
            (if (== (.Quantity (Utilities|Struct|BreakItemSetting _array_element)) 1)
              (Utilities|Array|RemoveIndex _inventorystock _array_index)
              (else
                (Utilities|Array|SetArrayElem _inventorystock _array_index (Utilities|Struct|MakeItemSetting (.ID (Utilities|Struct|BreakItemSetting _array_element)) (- (.Quantity (Utilities|Struct|BreakItemSetting _array_element)) 1))))))))
      (Transformation|AttachComponentToComponent (LocalVariables|GetDroppedItem) (Variables|Default|GetRightHand) (Variables|Default|GetSocketName) "SnapToTarget" "SnapToTarget" "SnapToTarget" true)
      (Class|SimplifiedVRChar|GripRight)
      (bind _asbp_item (Utilities|Casting|CastToBP_Item (Variables|Default|GetItemInHand)))
      (Transformation|SetMobility _asbp_item "Stationary"))
    (:6
      (bind _returnvalue_4 (Game|SpawnActorfromClass "/Game/Inventory/BP_Weapon.BP_Weapon_C" _returnvalue_2 "AlwaysSpawn" 0 0 :!label _label))
      (bind _output_get_2 (LocalVariables|SetWeponDropped _returnvalue_4))
      (Default|Dropped _output_get_2 ItemID)
      (for (_array_element_2 _array_index_2) (Variables|/Script/HeavenVR2.Inventory|GetInventoryStock (Variables|Default|GetInventory))
        (if (== (.ID (Utilities|Struct|BreakItemSetting _array_element_2)) ItemID)
          (if (== (.Quantity (Utilities|Struct|BreakItemSetting _array_element_2)) 1)
            (Utilities|Array|RemoveIndex _inventorystock_2 _array_index_2)
            (else
              (Utilities|Array|SetArrayElem _inventorystock_2 _array_index_2 (Utilities|Struct|MakeItemSetting (.ID (Utilities|Struct|BreakItemSetting _array_element_2)) (- (.Quantity (Utilities|Struct|BreakItemSetting _array_element_2)) 1)))))))
      (Transformation|AttachComponentToComponent (LocalVariables|GetWeponDropped) (Variables|Default|GetRightHand) (Variables|Default|GetSocketName) "SnapToTarget" "SnapToTarget" "SnapToTarget" true)
      (Class|SimplifiedVRChar|GripRight)
      (bind _asbp_weapon (Utilities|Casting|CastToBP_Weapon (Variables|Default|GetItemInHand)))
      (Transformation|SetMobility _asbp_weapon "Stationary"))
    (:7
      (goto _label))
    (:8
      (goto _label))))