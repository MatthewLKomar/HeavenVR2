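; Shrine actor that collects clue items from the VR player on overlap and triggers the game's ending.
; It filters clues from the player's inventory by data table, removes them (running the removal in two functions), and adds to its count.
; Each clue spawns as a dropped BP_Item in the next free of four spots, and filling the fourth spawns BP_Dialogue.
; Reaching the maximum count only prints a placeholder for a sound.
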(event OnComponentBeginOverlap(Collider)
  (params (OverlappedComponent :type Primitive%20Component%20Object%20Reference) (OtherActor :type Actor%20Object%20Reference) (OtherComp :type Primitive%20Component%20Object%20Reference) (OtherBodyIndex :type Integer) (bFromSweep :type Boolean) (SweepResult :type Hit%20Result%20Structure%20%28by%20ref%29))
  (bind _asbp_simplified_vrchar (Utilities|Casting|CastToBP_SimplifiedVRChar OtherActor))
  (bind _output_get (Variables|Default|SetPlayerRef _asbp_simplified_vrchar))
  (CallFunction|PlaceItemsonShrine _output_get)
  (if (== (Variables|Default|GetClueAmnt) (Variables|Default|GetMaxClueAmnt))
    (Development|PrintString "Play sound or some shit later")))

(fn ConstructionScript)

(fn TakeCluesfromPlayer
  (params (PlayerRef :type Simplified%20VR%20Char%20Object%20Reference))
  (LocalVariables|SetInventory (Variables|/Script/HeavenVR2.SimplifiedVRChar|GetInventory PlayerRef))
  (bind _returnvalue (Class|ClueShrine|GetCluesfromPlayer (Variables|/Script/HeavenVR2.Inventory|GetInventoryStock (Variables|/Script/HeavenVR2.SimplifiedVRChar|GetInventory PlayerRef)) (Variables|Default|GetItemDataTable)))
  (bind _output_get (Variables|Default|SetCluesFromPlayer _returnvalue))
  (CallFunction|RemoveCluefromInventory _output_get (LocalVariables|GetInventory))
  (return _output_get))

(fn RemoveCluefromInventory
  (params (Array :type Array%20of%20Item%20Setting%20Structures) (Inventory%20Component :type Inventory%20Object%20Reference))
  (for _array_element Array
    (Utilities|Array|RemoveItem (Variables|/Script/HeavenVR2.Inventory|GetInventoryStock Inventory%20Component) _array_element)
    (Class|Inventory|DecrementClue Inventory%20Component)))

(fn SpawnClues
  (params (ClueList :type Array%20of%20Item%20Setting%20Structures))
  (for _array_element ClueList
    (if (not (Variables|Default|GetSpot1Taken))
      (CallFunction|SpawnClue (.ID (Utilities|Struct|BreakItemSetting _array_element)) (Variables|Default|GetClueSpot1))
      (Variables|Default|SetSpot1Taken true)
      (elif (not (Variables|Default|GetSpot2Taken))
        (CallFunction|SpawnClue (.ID (Utilities|Struct|BreakItemSetting _array_element)) (Variables|Default|GetClueSpot2))
        (Variables|Default|SetSpot2Taken true)
        (elif (not (Variables|Default|GetSpot3Taken))
          (CallFunction|SpawnClue (.ID (Utilities|Struct|BreakItemSetting _array_element)) (Variables|Default|GetClueSpot3))
          (Variables|Default|SetSpot3Taken true)
          (elif (not (Variables|Default|GetSpot4Taken))
            (CallFunction|SpawnClue (.ID (Utilities|Struct|BreakItemSetting _array_element)) (Variables|Default|GetClueSpot4))
            (Variables|Default|SetSpot4Taken true)
            (CallFunction|EndGame)))))))

(fn SpawnClue
  (params (ID :type Integer) (Target :type Scene%20Component%20Object%20Reference))
  (bind _returnvalue (Game|SpawnActorfromClass "/Game/_blueprints/Inventory/BP_Item.BP_Item_C" (Math|Transform|MakeTransform (Transformation|GetWorldLocation Target)) "AlwaysSpawn" 0 0))
  (bind _output_get (Variables|Default|SetSpawnLocation _returnvalue))
  (Default|Dropped _output_get ID))

(fn PlaceItemsonShrine
  (params (PlayerRef :type Simplified%20VR%20Char%20Object%20Reference))
  (bind _output_get (CallFunction|TakeCluesfromPlayer PlayerRef))
  (Variables|Default|SetClueAmnt (+ (Utilities|Array|Length _output_get) (Variables|Default|GetClueAmnt)))
  (CallFunction|RemoveCluefromInventory _output_get (Variables|/Script/HeavenVR2.SimplifiedVRChar|GetInventory PlayerRef))
  (CallFunction|SpawnClues _output_get))

(fn EndGame
  (Game|SpawnActorfromClass "/Game/_blueprints/Z_Legacy/BP_Dialogue.BP_Dialogue_C" (Math|Transform|MakeTransform (Transformation|GetWorldLocation (Variables|Default|GetSpawner)) "0, 0, 0" "0.500000,0.500000,0.500000") "Undefined" 0 0))