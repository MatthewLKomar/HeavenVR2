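; Simplified VR player character with camera-relative forward movement, footstep sounds and tracked grip and trigger states.
; ItemID spawns the chosen inventory item or weapon in the right hand, grips it and decrements its stock, except for quest items.
; Tick destroys the UI actor unless only right grip is held with inventory enabled; the opening branch is an empty DoOnce.
; Hand-pose, pickup and release logic is disconnected.
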(event OnStep(FootStep)
  (Audio|PlaySoundatLocation 0 (Transformation|GetWorldLocation (Variables|Default|GetVRRoot)) "0, 0, 0" 1.0 1.0 0.0 0 0 0))

(event EventTick
  (params (DeltaSeconds :type Float%20%28single-precision%29))
  (bind _uiref (Variables|Default|GetUIRef))
  (if (Math|Boolean|ANDBoolean (Variables|Default|GetEnableInventory) (Variables|Default|GetRGripPressed) (not (Variables|Default|GetLTriggerPressed)) (not (Variables|Default|GetRTriggerPressed)) (not (Variables|Default|GetLGripPressed)))
    (Utilities|FlowControl|DoOnce false :!label _label)
    (elif (Utilities|IsValid _uiref)
      (Actor|DestroyActor _uiref)
      (goto _label Reset))))

(event EventBeginPlay
  (Class|HeadMountedDisplayFunctionLibrary|ResetOrientationandPosition (.y (Math|Vector|GetForwardVector (Variables|Default|GetCamera))) "OrientationAndPosition"))

(event Input|ActionEvents|InputActionEquip
  (params (Key :type Key%20Structure :default "None"))
  ;[0.9323 0.6341 0.4322] Input
  (:Released
    (Class|WidgetInteractionComponent|ReleasePointerKey (Variables|Default|GetRWidgetInteraction) "LeftMouseButton")))

(event Input|ActionEvents|InputActionTake
  (params (Key :type Key%20Structure :default "None"))
  ;[0.9323 0.6341 0.4322] Input
)

(event Input|ActionEvents|InputActionTriggerLeft
  (params (Key :type Key%20Structure :default "None"))
  (bind _lgrippressed (Variables|Default|GetLGripPressed))
  (bind _lefthand (Variables|Default|GetLeftHand))
  ;[0.9323 0.6341 0.4322] Input
  ;;[1 1 1] Pointing Logic
  (:Pressed
    (bind _pointstate (CallFunction|SetPointState _lefthand true _lgrippressed))
    (Variables|Default|SetLTriggerPressed _pointstate))
  (:Released
    (bind _pointstate_2 (CallFunction|SetPointState _lefthand false _lgrippressed))
    (Variables|Default|SetLTriggerPressed _pointstate_2)))

(event Input|ActionEvents|InputActionTriggerRight
  (params (Key :type Key%20Structure :default "None"))
  ;[0.9323 0.6341 0.4322] Input
  ;;[1 1 1] Pointing Logic
  (:Pressed
    (Variables|Default|SetRTriggerPressed true))
  (:Released
    (Variables|Default|SetRTriggerPressed false)))

(event Input|ActionEvents|InputActionGripRight
  (params (Key :type Key%20Structure :default "None"))
  ;[0.9323 0.6341 0.4322] Input
  ;;[1 1 1] Gripping Logic
  (:Pressed
    (Variables|Default|SetRGripPressed true))
  (:Released
    (Variables|Default|SetRGripPressed false)))

(event Input|ActionEvents|InputActionGripLeft
  (params (Key :type Key%20Structure :default "None"))
  ;[0.9323 0.6341 0.4322] Input
  ;;[1 1 1] Gripping Logic
  (:Pressed
    (Variables|Default|SetLGripPressed true))
  (:Released
    (Variables|Default|SetLGripPressed false)))

(event Input|AxisEvents|InputAxisMoveForward
  (params (AxisValue :type Float%20%28single-precision%29))
  (Pawn|Input|AddMovementInput (Math|Vector|GetForwardVector (Variables|Default|GetCamera)) AxisValue false))

(fn ConstructionScript)

(fn SetPointState
  (params (Hand :type Skeletal%20Mesh%20Component%20Object%20Reference) (TriggerPressed :type Boolean) (GripPressed :type Boolean) (WidgetInteractor :type Widget%20Interaction%20Component%20Object%20Reference)))

(fn SetGripState
  (params (GripPressed :type Boolean) (TriggerPressed :type Boolean) (Hand :type Skeletal%20Mesh%20Component%20Object%20Reference) (WidgetInteraction :type Widget%20Interaction%20Component%20Object%20Reference)))

(fn ItemID
  (params (ItemID :type Integer))
  (bind _inventory (Variables|Default|GetInventory))
  (bind _righthand (Variables|Default|GetRightHand))
  (bind _socketname (Variables|Default|GetSocketName))
  (bind _inventory_2 (Variables|Default|GetInventory))
  (bind _returnvalue (Transformation|GetSocketLocation _righthand _socketname))
  (bind _inventorystock (Variables|/Script/HeavenVR2.Inventory|GetInventoryStock _inventory))
  (bind _inventorystock_2 (Variables|/Script/HeavenVR2.Inventory|GetInventoryStock _inventory_2))
  (bind _returnvalue_2 (Math|Transform|MakeTransform _returnvalue))
  (switch int ItemID
    (:Default
      (bind _returnvalue_3 (Game|SpawnActorfromClass "/Game/_blueprints/Inventory/BP_Item.BP_Item_C" _returnvalue_2 "AlwaysSpawn" 0 0))
      (bind _output_get (LocalVariables|SetDroppedItem _returnvalue_3))
      (Default|Dropped _output_get ItemID)
      (for (_array_element _array_index) (Variables|/Script/HeavenVR2.Inventory|GetInventoryStock (Variables|Default|GetInventory))
        (if (== (.ID (Utilities|Struct|BreakItemSetting _array_element)) ItemID)
          ;[1 1 1] Remove Clues
          (if (not (Variables|/Script/HeavenVR2.Item|GetIsQuestItem (LocalVariables|GetDroppedItem)))
            (if (== (.Quantity (Utilities|Struct|BreakItemSetting _array_element)) 1)
              (Utilities|Array|RemoveIndex _inventorystock _array_index)
              (else
                (Utilities|Array|SetArrayElem _inventorystock _array_index (Utilities|Struct|MakeItemSetting (.ID (Utilities|Struct|BreakItemSetting _array_element)) (- (.Quantity (Utilities|Struct|BreakItemSetting _array_element)) 1))))))))
      (Transformation|AttachComponentToComponent (LocalVariables|GetDroppedItem) (Variables|Default|GetRightHand) (Variables|Default|GetSocketName) "SnapToTarget" "SnapToTarget" "SnapToTarget" true)
      (Class|SimplifiedVRChar|GripRight)
      (bind _asbp_item (Utilities|Casting|CastToBP_Item (Variables|Default|GetItemInHand)))
      (Transformation|SetMobility _asbp_item "Stationary"))
    (:6
      (bind _returnvalue_4 (Game|SpawnActorfromClass "/Game/_blueprints/Inventory/BP_Weapon.BP_Weapon_C" _returnvalue_2 "AlwaysSpawn" 0 0 :!label _label))
      (bind _output_get_2 (LocalVariables|SetWeponDropped _returnvalue_4))
      (Default|Dropped _output_get_2 ItemID)
      (for (_array_element_2 _array_index_2) (Variables|/Script/HeavenVR2.Inventory|GetInventoryStock (Variables|Default|GetInventory))
        (if (== (.ID (Utilities|Struct|BreakItemSetting _array_element_2)) ItemID)
          (if (== (.Quantity (Utilities|Struct|BreakItemSetting _array_element_2)) 1)
            (Utilities|Array|RemoveIndex _inventorystock_2 _array_index_2)
            (else
              (Utilities|Array|SetArrayElem _inventorystock_2 _array_index_2 (Utilities|Struct|MakeItemSetting (.ID (Utilities|Struct|BreakItemSetting _array_element_2)) (- (.Quantity (Utilities|Struct|BreakItemSetting _array_element_2)) 1)))))))
      (Transformation|AttachComponentToComponent (LocalVariables|GetWeponDropped) (Variables|Default|GetRightHand) (Variables|Default|GetSocketName) "SnapToTarget" "SnapToTarget" "SnapToTarget" true)
      (Class|SimplifiedVRChar|GripRight)
      (bind _asbp_weapon (Utilities|Casting|CastToBP_Weapon (Variables|Default|GetItemInHand)))
      (Transformation|SetMobility _asbp_weapon "Stationary"))
    (:7
      (goto _label))
    (:8
      (goto _label))))