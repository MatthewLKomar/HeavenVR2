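; Base creature Character that holds a CreatureInfo struct and provides shared health, movement speed and attack logic for child Blueprints.
; BeginPlay refreshes family-related details in that struct from the Chad and Childs references.
; Damage calls an overridable OnHurt, subtracts health into CreatureInfo, and triggers OnKilled once, which destroys the actor by default.
; Helpers switch walk speeds, toggle attack flags and play a random wake sound, while Setup, ThrowRangedItem and ShootProjectile are empty stubs.
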(event EventBeginPlay
  (Variables|Default|SetCreatureInfo (Utilities|Struct|MakeFCreatureDefinition (Utilities|Struct|MakeFCreatureData (.Species (Utilities|Struct|BreakFCreatureData (.CreatureDetails (Utilities|Struct|BreakFCreatureDefinition (Variables|Default|GetCreatureInfo))))) (.isMale (Utilities|Struct|BreakFCreatureData (.CreatureDetails (Utilities|Struct|BreakFCreatureDefinition (Variables|Default|GetCreatureInfo))))) (.Age (Utilities|Struct|BreakFCreatureData (.CreatureDetails (Utilities|Struct|BreakFCreatureDefinition (Variables|Default|GetCreatureInfo))))) (.Adult (Utilities|Struct|BreakFCreatureData (.CreatureDetails (Utilities|Struct|BreakFCreatureDefinition (Variables|Default|GetCreatureInfo))))) (not (Utilities|IsValid (Variables|Default|Getchad))) (!= (Utilities|Array|Length (Variables|Default|GetChilds)) 0) (.FoodLevel (Utilities|Struct|BreakFCreatureData (.CreatureDetails (Utilities|Struct|BreakFCreatureDefinition (Variables|Default|GetCreatureInfo))))) (.ThirstLevel (Utilities|Struct|BreakFCreatureData (.CreatureDetails (Utilities|Struct|BreakFCreatureDefinition (Variables|Default|GetCreatureInfo))))) (.isPredator (Utilities|Struct|BreakFCreatureData (.CreatureDetails (Utilities|Struct|BreakFCreatureDefinition (Variables|Default|GetCreatureInfo)))))) (.Health (Utilities|Struct|BreakFCreatureDefinition (Variables|Default|GetCreatureInfo))) (.Damage (Utilities|Struct|BreakFCreatureDefinition (Variables|Default|GetCreatureInfo))) (.CreatureInfo (Utilities|Struct|BreakFCreatureDefinition (Variables|Default|GetCreatureInfo))) (.UsePredefinedDmg (Utilities|Struct|BreakFCreatureDefinition (Variables|Default|GetCreatureInfo))))))

(event EventDamage
  (params (Damage :type Integer))
  (Utility|DamageCreature Damage))

(fn ConstructionScript)

(fn Setup)

(fn DamageCreature
  (params (Damage :type Integer))
  (Utilities|FlowControl|Sequence
    (:then_0
      (events|OnHurt Damage) ; This is to be overrided in ChildBP. This does sometihng cool when this gets hurt.
    )
    (:then_1
      (bind _output_get (Variables|Default|SetHealth (- (Variables|Default|GetHealth) Damage)))
      (if (and (<= _output_get 0) (not (Variables|Status|GetIsKill)))
        (Variables|Status|SetIsKill true)
        (Utility|SetHealth (Variables|Default|GetHealth) (Variables|Default|GetCreatureInfo))
        (events|OnKilled) ; This is to be overridded in childBP. This does something cool when thsi ies
        (else
          (Utility|SetHealth (Variables|Default|GetHealth) (Variables|Default|GetCreatureInfo)))))))

(fn OnHurt
  (params (Dmg :type Integer)))

(fn OnKilled
  (Actor|DestroyActor))

(fn SetAgroMoveSpeed
  (Variables|/Script/Engine.CharacterMovementComponent|SetMaxWalkSpeed (Variables|Character|GetCharacterMovement) (Variables|speed|GetAggroMoveSpeed)))

(fn SetDefaultMoveSpeed
  (Variables|/Script/Engine.CharacterMovementComponent|SetMaxWalkSpeed (Variables|Character|GetCharacterMovement) (Variables|Speed|GetDefaultMoveSpeed)))

(fn OnWake
  (Audio|PlaySoundatLocation (Utilities|Array|Get(acopy) (Variables|sound|GetSupriseSounds) (Math|Random|RandomIntegerinRange 0 (- (Utilities|Array|Length (Variables|sound|GetSupriseSounds)) 1))) (Transformation|GetActorLocation) "0, 0, 0" 1.0 1.0 0.0 0 0 0))

(fn MeleeAttack
  (Variables|Status|SetIsMeleeAttack true))

(fn RangedAttack
  (Variables|Status|SetIsRangedAttack true))

(fn OnRangedAttackOver
  (Variables|Status|SetIsRangedAttack false))

(fn OnMeleeAttackOver
  (Variables|Status|SetIsMeleeAttack false))

(fn ThrowRangedItem)

(fn ShootProjectile)

(fn SetHealth
  (params (Health :type Integer) (CreatureInfo :type F%20Creature%20Definition%20Structure))
  (Variables|Default|SetCreatureInfo (Utilities|Struct|MakeFCreatureDefinition (.creaturedetails CreatureInfo) Health (.damage CreatureInfo) (.creatureinfo CreatureInfo) (.usepredefineddmg CreatureInfo))))

(fn SetAttackSpeed
  (Variables|/Script/Engine.CharacterMovementComponent|SetMaxWalkSpeed (Variables|Character|GetCharacterMovement) (Variables|Speed|GetAttackSpeed)))