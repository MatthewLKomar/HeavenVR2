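; Spawner actor that creates a flock of BP_Creature animals at BeginPlay.
; It spawns a lead creature ("Chad") at its own location, then spawns followers at random navigable points within its capsule radius.
; Each follower receives the Chad reference and a default controller, and the inclusive loop yields one more than AnimalsInFlock.
; The leader and follower array are registered as a key-value pair in Flock's Flocks map.
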(event EventBeginPlay
  (bind _returnvalue (Game|SpawnActorfromClass "/Game/_blueprints/Creatures/BP_Creature.BP_Creature_C" (Math|Transform|MakeTransform (Transformation|GetActorLocation) "0, 0, 0" "1,1,1") "AdjustIfPossibleButAlwaysSpawn" 0 0 0 0 0 0))
  (bind _animals1 (CallFunction|CreateAnimals (Variables|Default|GetAnimalsInFlock) _returnvalue))
  (Utilities|Map|Add (Utilities|Struct|BreakF_CreatureFlocks (Variables|Default|GetFlock)) _returnvalue (Utilities|Struct|MakeF_CreatureFollowers _animals1)))

(fn ConstructionScript)

(fn CreateAnimals
  (params (LastIndex :type Integer) (chad :type BP%20Creature%20Object%20Reference))
  (for _index (range 0 LastIndex)
    (bind _returnvalue (Game|SpawnActorfromClass "/Game/_blueprints/Creatures/BP_Creature.BP_Creature_C" (Math|Transform|MakeTransform (.RandomLocation (Class|NavigationSystemV1|GetRandomPointinNavigableRadius (Transformation|GetActorLocation) (Variables|/Script/Engine.CapsuleComponent|GetCapsuleRadius (Variables|Default|GetCapsule)) 0 0)) "0, 0, 0" "1,1,1") "Undefined" 0 0 0 0 chad 0))
    (Pawn|SpawnDefaultController _returnvalue)
    (Utilities|Array|Add (LocalVariables|GetAnimals) _returnvalue))
  (return (LocalVariables|GetAnimals)))