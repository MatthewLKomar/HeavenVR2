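; VR player character with camera-relative movement, two-hand gripping, item pickup and an inventory.
; Grip and trigger states set hand animation poses and the right widget pointer's debug beam.
; When inventory is enabled, holding only right grip spawns its UI on the left hand.
; Take stores held items and counts quest clues; ItemID spawns chosen items or weapons into the right hand, decrementing stock except quest items.
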(event OnStep(FootStep)
  (Audio|PlaySoundatLocation 0 (Transformation|GetWorldLocation (Variables|Default|GetVRRoot)) "0, 0, 0" 1.0 1.0 0.0 0 0 0))

(event EventTick
  (params (DeltaSeconds :type Float%20%28single-precision%29))
  (if (Math|Boolean|ANDBoolean (Variables|Default|GetEnableInventory) (Variables|Default|GetRGripPressed) (not (Variables|Default|GetLTriggerPressed)) (not (Variables|Default|GetRTriggerPressed)) (not (Variables|Default|GetLGripPressed)))
    (Utilities|FlowControl|DoOnce false :!label _label
      (:Completed
        (bind _returnvalue (Class|SimplifiedVRChar|SpawnInventory (Variables|Default|GetLeftHand) 0 false))
        (Variables|Default|SetUIRef _returnvalue)))
    (elif (Utilities|IsValid (Variables|Default|GetUIRef))
      (Actor|DestroyActor (Variables|Default|GetUIRef))
      (goto _label Reset))))

(event EventBeginPlay
  (Class|HeadMountedDisplayFunctionLibrary|ResetOrientationandPosition (.y (Math|Vector|GetForwardVector (Variables|Default|GetCamera))) "OrientationAndPosition"))

(event Input|ActionEvents|InputActionEquip
  (params (Key :type Key%20Structure :default "None"))
  (bind _rwidgetinteraction (Variables|Default|GetRWidgetInteraction))
  ;[0.9323 0.6341 0.4322] Input
  (:Pressed
    (Class|WidgetInteractionComponent|PressPointerKey _rwidgetinteraction "LeftMouseButton"))
  (:Released
    (Class|WidgetInteractionComponent|ReleasePointerKey _rwidgetinteraction "LeftMouseButton")))

(event Input|ActionEvents|InputActionTake
  (params (Key :type Key%20Structure :default "None"))
  ;[0.9323 0.6341 0.4322] Input
  (:Pressed
    (bind _asbp_item (Utilities|Casting|CastToBP_Item (Variables|Default|GetHeldObject)))
    (Utilities|IsValid _asbp_item
      (:Is%20Valid
        (bind (_id _questitem _amountofitems) (Class|Item|PickUp _asbp_item))
        (if _questitem
          (Class|Inventory|IncrementClue (Variables|Default|GetInventory)))
        (bind _returnvalue (Class|Inventory|AddItemtoInventory (Variables|Default|GetInventory) _id _amountofitems))
        (if _returnvalue
          (Actor|DestroyActor (Variables|Default|GetHeldObject)))))))

(event Input|ActionEvents|InputActionTriggerLeft
  (params (Key :type Key%20Structure :default "None"))
  (bind _lgrippressed (Variables|Default|GetLGripPressed))
  (bind _lefthand (Variables|Default|GetLeftHand))
  ;[0.9323 0.6341 0.4322] Input
  ;;[1 1 1] Pointing Logic
  (:Pressed
    (bind _pointstate (CallFunction|SetPointState _lefthand true _lgrippressed))
    (Variables|Default|SetLTriggerPressed _pointstate))
  (:Released
    (bind _pointstate_2 (CallFunction|SetPointState _lefthand false _lgrippressed))
    (Variables|Default|SetLTriggerPressed _pointstate_2)))

(event Input|ActionEvents|InputActionTriggerRight
  (params (Key :type Key%20Structure :default "None"))
  (bind _rwidgetinteraction (Variables|Default|GetRWidgetInteraction))
  (bind _rgrippressed (Variables|Default|GetRGripPressed))
  (bind _righthand (Variables|Default|GetRightHand))
  ;[0.9323 0.6341 0.4322] Input
  ;;[1 1 1] Pointing Logic
  (:Pressed
    (bind _pointstate (CallFunction|SetPointState _righthand true _rgrippressed _rwidgetinteraction))
    (Variables|Default|SetRTriggerPressed _pointstate))
  (:Released
    (bind _pointstate_2 (CallFunction|SetPointState _righthand false _rgrippressed _rwidgetinteraction))
    (Variables|Default|SetRTriggerPressed _pointstate_2)))

(event Input|ActionEvents|InputActionGripRight
  (params (Key :type Key%20Structure :default "None"))
  (bind _iteminhand (Variables|Default|GetItemInHand))
  (bind _rwidgetinteraction (Variables|Default|GetRWidgetInteraction))
  (bind _righthand (Variables|Default|GetRightHand))
  (bind _rtriggerpressed (Variables|Default|GetRTriggerPressed))
  ;[0.9323 0.6341 0.4322] Input
  ;;[1 1 1] Gripping Logic
  (:Pressed
    (bind _gripstate (CallFunction|SetGripState true _rtriggerpressed _righthand _rwidgetinteraction))
    (Variables|Default|SetRGripPressed _gripstate)
    (Class|SimplifiedVRChar|GripRight)
    (bind _asbp_item (Utilities|Casting|CastToBP_Item _iteminhand))
    (Utilities|IsValid _asbp_item
      (:Is%20Valid
        (Transformation|SetMobility _asbp_item "Stationary"))))
  (:Released
    (bind _gripstate_2 (CallFunction|SetGripState false _rtriggerpressed _righthand _rwidgetinteraction))
    (Variables|Default|SetRGripPressed _gripstate_2)
    (bind _asbp_item_2 (Utilities|Casting|CastToBP_Item _iteminhand))
    (Utilities|IsValid _asbp_item_2
      (:Is%20Valid
        (Transformation|SetMobility _asbp_item_2 "Movable")
        (Transformation|DetachFromActor _asbp_item_2 "KeepWorld" "KeepWorld" "KeepWorld")
        (Class|SimplifiedVRChar|ReleaseRight)))))

(event Input|ActionEvents|InputActionGripLeft
  (params (Key :type Key%20Structure :default "None"))
  (bind _lefthand (Variables|Default|GetLeftHand))
  (bind _ltriggerpressed (Variables|Default|GetLTriggerPressed))
  (bind _iteminhand (Variables|Default|GetItemInHand))
  ;[0.9323 0.6341 0.4322] Input
  ;;[1 1 1] Gripping Logic
  (:Pressed
    (bind _gripstate (CallFunction|SetGripState true _ltriggerpressed _lefthand))
    (Variables|Default|SetLGripPressed _gripstate)
    (Class|SimplifiedVRChar|GripLeft)
    (bind _asbp_item (Utilities|Casting|CastToBP_Item _iteminhand))
    (Utilities|IsValid _asbp_item
      (:Is%20Valid
        (Transformation|SetMobility _asbp_item "Stationary"))))
  (:Released
    (bind _gripstate_2 (CallFunction|SetGripState false _ltriggerpressed _lefthand))
    (Variables|Default|SetLGripPressed _gripstate_2)
    (bind _asbp_item_2 (Utilities|Casting|CastToBP_Item _iteminhand))
    (Utilities|IsValid _asbp_item_2
      (:Is%20Valid
        (Transformation|SetMobility _asbp_item_2 "Movable")
        (Class|SimplifiedVRChar|ReleaseLeft)))))

(event Input|AxisEvents|InputAxisMoveForward
  (params (AxisValue :type Float%20%28single-precision%29))
  (Pawn|Input|AddMovementInput (Math|Vector|GetForwardVector (Variables|Default|GetCamera)) AxisValue false))

(fn ConstructionScript)

(fn SetPointState
  (params (Hand :type Skeletal%20Mesh%20Component%20Object%20Reference) (TriggerPressed :type Boolean) (GripPressed :type Boolean) (WidgetInteractor :type Widget%20Interaction%20Component%20Object%20Reference))
  (bind _asbp_hand_anim (Utilities|Casting|CastToBP_Hand_Anim (Components|SkeletalMesh|GetAnimInstance Hand)))
  (LocalVariables|SetHandAnim _asbp_hand_anim)
  (if TriggerPressed
    ;[1 1 1] What to do if we're pointing and are we gripping?
    (if GripPressed
      (Variables|/Game/_Assets/CustomHand/Anim/BP_Hand_Anim.BP_Hand_Anim_C|SetOpen (LocalVariables|GetHandAnim) 3.0)
      (else
        (Variables|/Game/_Assets/CustomHand/Anim/BP_Hand_Anim.BP_Hand_Anim_C|SetOpen (LocalVariables|GetHandAnim) 1.0)))
    (Utilities|IsValid WidgetInteractor
      (:Is%20Valid
        (Variables|/Script/UMG.WidgetInteractionComponent|SetbShowDebug WidgetInteractor false)))
    (elif GripPressed
      (Variables|/Game/_Assets/CustomHand/Anim/BP_Hand_Anim.BP_Hand_Anim_C|SetOpen (LocalVariables|GetHandAnim) 2.0)
      (Utilities|IsValid WidgetInteractor
        (:Is%20Valid
          (Variables|/Script/UMG.WidgetInteractionComponent|SetbShowDebug WidgetInteractor true)))
      (else
        (Variables|/Game/_Assets/CustomHand/Anim/BP_Hand_Anim.BP_Hand_Anim_C|SetOpen (LocalVariables|GetHandAnim) 0.0)
        (Utilities|IsValid WidgetInteractor
          (:Is%20Valid
            (Variables|/Script/UMG.WidgetInteractionComponent|SetbShowDebug WidgetInteractor false))))))
  (return TriggerPressed))

(fn SetGripState
  (params (GripPressed :type Boolean) (TriggerPressed :type Boolean) (Hand :type Skeletal%20Mesh%20Component%20Object%20Reference) (WidgetInteraction :type Widget%20Interaction%20Component%20Object%20Reference))
  (bind _asbp_hand_anim (Utilities|Casting|CastToBP_Hand_Anim (Components|SkeletalMesh|GetAnimInstance Hand)))
  (LocalVariables|SetHandAnim _asbp_hand_anim)
  (if GripPressed
    (if TriggerPressed
      (Variables|/Game/_Assets/CustomHand/Anim/BP_Hand_Anim.BP_Hand_Anim_C|SetOpen (LocalVariables|GetHandAnim) 3.0)
      (Utilities|IsValid WidgetInteraction
        (:Is%20Valid
          (Variables|/Script/UMG.WidgetInteractionComponent|SetbShowDebug WidgetInteraction false :!label _label))
        (:Is%20Not%20Valid
          _))
      (else
        (Variables|/Game/_Assets/CustomHand/Anim/BP_Hand_Anim.BP_Hand_Anim_C|SetOpen (LocalVariables|GetHandAnim) 2.0)
        (Utilities|IsValid WidgetInteraction
          (:Is%20Valid
            (Variables|/Script/UMG.WidgetInteractionComponent|SetbShowDebug WidgetInteraction true))
          (:Is%20Not%20Valid
            _))))
    (elif TriggerPressed
      (Variables|/Game/_Assets/CustomHand/Anim/BP_Hand_Anim.BP_Hand_Anim_C|SetOpen (LocalVariables|GetHandAnim) 1.0)
      (Utilities|IsValid WidgetInteraction
        (:Is%20Valid
          (goto _label))
        (:Is%20Not%20Valid
          _))
      (else
        (Variables|/Game/_Assets/CustomHand/Anim/BP_Hand_Anim.BP_Hand_Anim_C|SetOpen (LocalVariables|GetHandAnim) 0.0)
        (Utilities|IsValid WidgetInteraction
          (:Is%20Valid
            (goto _label))
          (:Is%20Not%20Valid
            _)))))
  (return GripPressed))

(fn ItemID
  (params (ItemID :type Integer))
  (bind _inventory (Variables|Default|GetInventory))
  (bind _righthand (Variables|Default|GetRightHand))
  (bind _socketname (Variables|Default|GetSocketName))
  (bind _inventory_2 (Variables|Default|GetInventory))
  (bind _returnvalue (Transformation|GetSocketLocation _righthand _socketname))
  (bind _inventorystock (Variables|/Script/HeavenVR2.Inventory|GetInventoryStock _inventory))
  (bind _inventorystock_2 (Variables|/Script/HeavenVR2.Inventory|GetInventoryStock _inventory_2))
  (bind _returnvalue_2 (Math|Transform|MakeTransform _returnvalue))
  (switch int ItemID
    (:Default
      (bind _returnvalue_3 (Game|SpawnActorfromClass "/Game/_blueprints/Inventory/BP_Item.BP_Item_C" _returnvalue_2 "AlwaysSpawn" 0 0))
      (bind _output_get (LocalVariables|SetDroppedItem _returnvalue_3))
      (Default|Dropped _output_get ItemID)
      (for (_array_element _array_index) (Variables|/Script/HeavenVR2.Inventory|GetInventoryStock (Variables|Default|GetInventory))
        (if (== (.ID (Utilities|Struct|BreakItemSetting _array_element)) ItemID)
          ;[1 1 1] Remove Clues
          (if (not (Variables|/Script/HeavenVR2.Item|GetIsQuestItem (LocalVariables|GetDroppedItem)))
            (if (== (.Quantity (Utilities|Struct|BreakItemSetting _array_element)) 1)
              (Utilities|Array|RemoveIndex _inventorystock _array_index)
              (else
                (Utilities|Array|SetArrayElem _inventorystock _array_index (Utilities|Struct|MakeItemSetting (.ID (Utilities|Struct|BreakItemSetting _array_element)) (- (.Quantity (Utilities|Struct|BreakItemSetting _array_element)) 1))))))))
      (Transformation|AttachComponentToComponent (LocalVariables|GetDroppedItem) (Variables|Default|GetRightHand) (Variables|Default|GetSocketName) "SnapToTarget" "SnapToTarget" "SnapToTarget" true)
      (Class|SimplifiedVRChar|GripRight)
      (bind _asbp_item (Utilities|Casting|CastToBP_Item (Variables|Default|GetItemInHand)))
      (Transformation|SetMobility _asbp_item "Stationary"))
    (:6
      (bind _returnvalue_4 (Game|SpawnActorfromClass "/Game/_blueprints/Inventory/BP_Weapon.BP_Weapon_C" _returnvalue_2 "AlwaysSpawn" 0 0 :!label _label))
      (bind _output_get_2 (LocalVariables|SetWeponDropped _returnvalue_4))
      (Default|Dropped _output_get_2 ItemID)
      (for (_array_element_2 _array_index_2) (Variables|/Script/HeavenVR2.Inventory|GetInventoryStock (Variables|Default|GetInventory))
        (if (== (.ID (Utilities|Struct|BreakItemSetting _array_element_2)) ItemID)
          (if (== (.Quantity (Utilities|Struct|BreakItemSetting _array_element_2)) 1)
            (Utilities|Array|RemoveIndex _inventorystock_2 _array_index_2)
            (else
              (Utilities|Array|SetArrayElem _inventorystock_2 _array_index_2 (Utilities|Struct|MakeItemSetting (.ID (Utilities|Struct|BreakItemSetting _array_element_2)) (- (.Quantity (Utilities|Struct|BreakItemSetting _array_element_2)) 1)))))))
      (Transformation|AttachComponentToComponent (LocalVariables|GetWeponDropped) (Variables|Default|GetRightHand) (Variables|Default|GetSocketName) "SnapToTarget" "SnapToTarget" "SnapToTarget" true)
      (Class|SimplifiedVRChar|GripRight)
      (bind _asbp_weapon (Utilities|Casting|CastToBP_Weapon (Variables|Default|GetItemInHand)))
      (Transformation|SetMobility _asbp_weapon "Stationary"))
    (:7
      (goto _label))
    (:8
      (goto _label))))