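; BP_Cart is a cart actor that rides along the spline of a referenced track.
; On BeginPlay it scales the CartMover timeline by Duration, applies a start offset and calls Activate, which toggles between moving and stopping via ActiveCart.
; Each timeline update maps Alpha to distance along the spline, setting world location and rotation.
; It also binds Escape to quit the game.
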(event Custom|MoveCart
  (bind _alpha (Timeline|CartMover Play)
    (:Update
      (Variables|Default|SetAlpha _alpha)
      (Transformation|SetActorLocationAndRotation (Spline|GetLocationatDistanceAlongSpline (Variables|/Game/_blueprints/BP_Track.BP_Track_C|GetUseful%20Spline (Variables|Default|GetTrackRef)) (Math|Float|Lerp 0.0 (Spline|GetSplineLength (Variables|/Game/_blueprints/BP_Track.BP_Track_C|GetUseful%20Spline (Variables|Default|GetTrackRef))) (Variables|Default|GetAlpha)) "World") (Spline|GetRotationatDistanceAlongSpline (Variables|/Game/_blueprints/BP_Track.BP_Track_C|GetUseful%20Spline (Variables|Default|GetTrackRef)) (Math|Float|Lerp 0.0 (Spline|GetSplineLength (Variables|/Game/_blueprints/BP_Track.BP_Track_C|GetUseful%20Spline (Variables|Default|GetTrackRef))) (Variables|Default|GetAlpha)) "World")))))

(event Custom|Stop
  (bind _alpha (Timeline|CartMover Stop)
    (:Update
      (Variables|Default|SetAlpha _alpha)
      (Transformation|SetActorLocationAndRotation (Spline|GetLocationatDistanceAlongSpline (Variables|/Game/_blueprints/BP_Track.BP_Track_C|GetUseful%20Spline (Variables|Default|GetTrackRef)) (Math|Float|Lerp 0.0 (Spline|GetSplineLength (Variables|/Game/_blueprints/BP_Track.BP_Track_C|GetUseful%20Spline (Variables|Default|GetTrackRef))) (Variables|Default|GetAlpha)) "World") (Spline|GetRotationatDistanceAlongSpline (Variables|/Game/_blueprints/BP_Track.BP_Track_C|GetUseful%20Spline (Variables|Default|GetTrackRef)) (Math|Float|Lerp 0.0 (Spline|GetSplineLength (Variables|/Game/_blueprints/BP_Track.BP_Track_C|GetUseful%20Spline (Variables|Default|GetTrackRef))) (Variables|Default|GetAlpha)) "World")))))

(event Custom|Activate
  (if (Variables|Default|GetActiveCart)
    (CallFunction|MoveCart)
    (Variables|Default|SetActiveCart false)
    (else
      (CallFunction|Stop)
      (Variables|Default|SetActiveCart true))))

(event EventBeginPlay
  (Components|Timeline|SetPlayRate (Variables|Default|GetCartMover) (/ 1.0 (Variables|Default|GetDuration)))
  (Components|Timeline|SetNewTime (Variables|Default|GetCartMover) (Variables|Default|GetCartStartOffset))
  (CallFunction|Activate))

(event Input|KeyboardEvents|Escape
  (params (Key :type Key%20Structure :default "None"))
  (:Pressed
    (Game|QuitGame 0 "Quit" true)))

(fn ConstructionScript)